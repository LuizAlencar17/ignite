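; Damageable enemy that takes a random skeletal mesh from its Meshs array on BeginPlay and shows a health bar widget.
; Each hit re-links the BP_HealthBar widget to this enemy, subtracts Health, and refreshes the bar while Health is not negative.
; Below zero it plays an explosion sound at world origin, spawns an emitter at the mesh, increments FirstPersonCharacter's EnemiesDie count and destroys itself.
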(event `self.ReceiveBeginPlay`
  (`SkinnedMeshComponent.SetSkinnedAssetAndUpdate` (`self.Mesh`) (`|GetArrayItem` (`self.Meshs`) (`KismetMathLibrary.RandomIntegerInRange` 0 5)) true))

(event `self.ReceiveAnyDamage`
  (params (Damage :type "Float (single-precision)") (DamageType :type "DamageType Object Reference") (InstigatedBy :type "Controller Object Reference") (DamageCauser :type "Actor Object Reference"))
  ;[1 1 1] Health Controller
  (`|ExecutionSequence`
    (:`then_0`
      (bind _asbp_health_bar (cast `/Game/MyThings/Blueprints/BP_HealthBar` (`WidgetComponent.GetUserWidgetObject` (`self.Widget`))))
      (bind _output_get (set `self.EnemyHealthBarWidget` _asbp_health_bar))
      (set `/Game/MyThings/Blueprints/BP_HealthBar.Enemy` self _output_get))
    (:`then_1`
      (bind _output_get_2 (set `self.Health` (- (`self.Health`) Damage)))
      (if (< _output_get_2 0.0)
        (`GameplayStatics.PlaySoundAtLocation` "/Game/StarterContent/Audio/Explosion01.Explosion01" (0.0 0.0 0.0) (struct) 1.0 1.0 0.0 null null null)
        (`GameplayStatics.SpawnEmitterAtLocation` "/Game/StarterContent/Particles/P_Explosion.P_Explosion" (`SceneComponent.K2_GetComponentLocation` (`self.Mesh`)) (struct) (2.0 2.0 2.0))
        (bind _asfirst_person_character (cast `/Game/MyThings/Blueprints/FirstPersonCharacter` (`GameplayStatics.GetPlayerCharacter` 0)))
        (set `/Game/MyThings/Blueprints/FirstPersonCharacter.EnemiesDie` (+ (`/Game/MyThings/Blueprints/FirstPersonCharacter.EnemiesDie` _asfirst_person_character) 1) _asfirst_person_character)
        (`self.K2_DestroyActor`)
        (else
          (`/Game/MyThings/Blueprints/BP_HealthBar.Update Health` (`self.EnemyHealthBarWidget`)))))))

(fn `UserConstructionScript`)